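; BP_CameraDirector is a Gameplay Cameras director that selects camera rigs for BP_LttnCharacter.
; On activation it sets persistent global collision-offset and base-default rigs and caches the owning character.
; Each run feeds the character's camera properties into a Chooser table and activates the resulting rig without forcing a new instance.
; A trailing first-person style check currently does nothing.
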(event EventRunCameraDirector
  (params (DeltaTime :type Float%20%28single-precision%29) (EvaluationContextOwner :type Object%20Object%20Reference) (Params :type Blueprint%20Camera%20Director%20Evaluation%20Params%20Structure%20%28by%20ref%29))
  (bind _character (Variables|Default|GetCharacter))
  (bind _returnvalue (Class|LttnCharacter|GetPropertiesCamera _character))
  (bind _result (|EvaluateChooser2 _returnvalue)
    (:execute
      (Class|BlueprintCameraDirectorEvaluator|ActivateCameraRig _result false)
      (if (Utilities|Enum|Equal(Enum) (.CameraStyle (Utilities|Struct|BreakPropertiesForCamera _returnvalue)) "FirstP")
        _))))

(event EventActivateCameraDirector
  (params (EvaluationContextOwner :type Object%20Object%20Reference) (Params :type Blueprint%20Camera%20Director%20Activate%20Params%20Structure%20%28by%20ref%29))
  (Class|BlueprintCameraDirectorEvaluator|ActivatePersistentGlobalCameraRig "/Game/Blueprints/Cameras/Rigs/CameraRig_CollisionOffset.CameraRig_CollisionOffset")
  (Class|BlueprintCameraDirectorEvaluator|ActivatePersistentBaseCameraRig "/Game/Blueprints/Cameras/Rigs/CameraRig_BaseDefaults.CameraRig_BaseDefaults")
  (bind _asbp_lttn_character (Utilities|Casting|CastToBP_LttnCharacter (Class|BlueprintCameraDirectorEvaluator|FindEvaluationContextOwnerActor "/Script/Engine.Actor")))
  (Variables|Default|SetCharacter _asbp_lttn_character))