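; Character Blueprint for Lttn that exposes move input, weapon location and overlap hooks.
; Sphere overlaps forward to OverlapStart and OverlapEnd, with a toggle for overlap events, and getters wrap IA_Move values and the Billboard's location.
; RagdollStart stops movement, disables capsule and mesh collision, and simulates physics from the pelvis down.
; BeginPlay carries apparent test code that damages one name-matched instance after a delay.
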(event OnComponentBeginOverlap(Sphere)
  (params (OverlappedComponent :type Primitive%20Component%20Object%20Reference) (OtherActor :type Actor%20Object%20Reference) (OtherComp :type Primitive%20Component%20Object%20Reference) (OtherBodyIndex :type Integer) (bFromSweep :type Boolean) (SweepResult :type Hit%20Result%20Structure%20%28by%20ref%29))
  (Class|LttnCharacter|OverlapStart OtherActor))

(event OnComponentEndOverlap(Sphere)
  (params (OverlappedComponent :type Primitive%20Component%20Object%20Reference) (OtherActor :type Actor%20Object%20Reference) (OtherComp :type Primitive%20Component%20Object%20Reference) (OtherBodyIndex :type Integer))
  (Class|LttnCharacter|OverlapEnd OtherActor))

(event EventTick
  (params (DeltaSeconds :type Float%20%28single-precision%29)))

(event EventBeginPlay
  (bind _self self)
  (Utilities|FlowControl|Delay 5.0)
  (if (Utilities|Enum|Equal(Enum) (Utilities|GetObjectName self) "BP_LttnCharacter_C_1")
    (Game|Damage|ApplyPointDamage _self 1e+01 (Math|Vector|GetForwardVector (Transformation|GetActorRotation)) (Collision|MakeHitResult true false 0.0 0.0 "0, 0, 0" "0, 0, 0" "0,0,1" "0,0,1" 0 0) 0 _self)))

(event EventEnableCollisionSphere
  (params (bEnabled :type Boolean))
  (Variables|/Script/Engine.PrimitiveComponent|SetbGenerateOverlapEvents (Variables|Default|GetSphere) bEnabled))

(fn ConstructionScript)

(fn GetIAMoveWorldVector
  (return (Input|EnhancedActionValues|GetIA_Move_WorldSpace)))

(fn GetIAMoveVector
  (return (Input|EnhancedActionValues|GetIA_Move)))

(fn GetWeaponLocation
  (return (Transformation|GetWorldLocation (Variables|Default|GetBillboard))))

(fn RagdollStart
  (bind _mesh (Variables|Character|GetMesh))
  (Pawn|Components|CharacterMovement|SetMovementMode (Variables|Character|GetCharacterMovement) "MOVE_None" 0)
  (Collision|SetCollisionEnabled (Variables|Default|GetCapsuleComponent) "NoCollision")
  (Collision|SetCollisionObjectType _mesh "ECC_PhysicsBody")
  (Collision|SetCollisionEnabled _mesh "NoCollision")
  (Class|SkeletalMeshComponent|SetAllBodiesBelowSimulatePhysics (Variables|Character|GetMesh) (Utilities|Name|MakeLiteralName "pelvis") true true))