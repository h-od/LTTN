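; BP_Door1 is a sliding door actor whose box trigger calls NotifyActor when an actor enters or leaves.
; Open chains two timelines to move Cube along relative X, then Y, then sets IsOpen.
; Close runs the Y timeline before the X one, then calls OnDoorCloseComplete.
; Timeline tracks feed the Lerps' A input, with B at zero and IntOpenX or IntOpenY as fixed alpha, so they scale the curve output.
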(event OnComponentBeginOverlap(Box)
  (params (OverlappedComponent :type Primitive%20Component%20Object%20Reference) (OtherActor :type Actor%20Object%20Reference) (OtherComp :type Primitive%20Component%20Object%20Reference) (OtherBodyIndex :type Integer) (bFromSweep :type Boolean) (SweepResult :type Hit%20Result%20Structure%20%28by%20ref%29))
  (Class|Door|NotifyActor OtherActor true))

(event OnComponentEndOverlap(Box)
  (params (OverlappedComponent :type Primitive%20Component%20Object%20Reference) (OtherActor :type Actor%20Object%20Reference) (OtherComp :type Primitive%20Component%20Object%20Reference) (OtherBodyIndex :type Integer))
  (Class|Door|NotifyActor OtherActor false))

(event EventOpen
  (bind _cube (Variables|Default|GetCube))
  (bind _cube_2 (Variables|Default|GetCube))
  (bind _relativelocation (Variables|/Script/Engine.SceneComponent|GetRelativeLocation _cube))
  (bind _relativelocation_2 (Variables|/Script/Engine.SceneComponent|GetRelativeLocation _cube_2))
  (bind _zeroto1 (Timeline|OpenX_2 Play)
    (:Update
      (Transformation|SetRelativeLocation _cube (Math|Vector|MakeVector (Math|Float|Lerp _zeroto1 0.0 (Variables|Default|GetIntOpenX)) (.y _relativelocation) (.z _relativelocation)) false false))
    (:Finished
      (bind _zeroto1_2 (Timeline|OpenY_2 Play)
        (:Update
          (Transformation|SetRelativeLocation _cube_2 (Math|Vector|MakeVector (.x _relativelocation_2) (Math|Float|Lerp _zeroto1_2 0.0 (Variables|Default|GetIntOpenY)) (.z _relativelocation_2)) false false))
        (:Finished
          (Variables|Default|SetIsOpen true))))))

(event EventClose
  (bind _cube (Variables|Default|GetCube))
  (bind _cube_2 (Variables|Default|GetCube))
  (bind _relativelocation (Variables|/Script/Engine.SceneComponent|GetRelativeLocation _cube))
  (bind _relativelocation_2 (Variables|/Script/Engine.SceneComponent|GetRelativeLocation _cube_2))
  (bind _zeroto1 (Timeline|CloseY_1 Play)
    (:Update
      (Transformation|SetRelativeLocation _cube_2 (Math|Vector|MakeVector (.x _relativelocation_2) (Math|Float|Lerp _zeroto1 0.0 (Variables|Default|GetIntOpenY)) (.z _relativelocation_2)) false false))
    (:Finished
      (bind _1tozero (Timeline|CloseX_1 Play)
        (:Update
          (Transformation|SetRelativeLocation _cube (Math|Vector|MakeVector (Math|Float|Lerp _1tozero 0.0 (Variables|Default|GetIntOpenX)) (.y _relativelocation) (.z _relativelocation)) false false))
        (:Finished
          (Class|Door|OnDoorCloseComplete))))))

(fn ConstructionScript)