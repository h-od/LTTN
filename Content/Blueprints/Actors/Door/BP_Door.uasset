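; Door actor that slides its Cube mesh open and closed in two axis steps when enabled.
; Open chains timelines along X then Y, but only for non-exterior doors; Close runs Y then X, with separate exterior and interior timelines and offsets.
; IsOpen updates after the final step.
; OnDoorCloseComplete fires when closing finishes, or immediately if Close is called while disabled.
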(event EventOpen
  (bind _cube (Variables|Default|GetCube))
  (bind _cube_2 (Variables|Default|GetCube))
  (bind _relativelocation (Variables|/Script/Engine.SceneComponent|GetRelativeLocation _cube))
  (bind _relativelocation_2 (Variables|/Script/Engine.SceneComponent|GetRelativeLocation _cube_2))
  (if (Variables|Default|GetEnabled)
    (if (not (Variables|Default|GetIsOpen))
      (if (not (Variables|Default|GetIsExt))
        (bind _zeroto1 (Timeline|OpenX_2 Play)
          (:Update
            (Transformation|SetRelativeLocation _cube (Math|Vector|MakeVector (Math|Float|Lerp _zeroto1 0.0 (Variables|Default|GetIntOpenX)) (.y _relativelocation) (.z _relativelocation)) false false))
          (:Finished
            (bind _zeroto1_2 (Timeline|OpenY_2 Play)
              (:Update
                (Transformation|SetRelativeLocation _cube_2 (Math|Vector|MakeVector (.x _relativelocation_2) (Math|Float|Lerp _zeroto1_2 0.0 (Variables|Default|GetIntOpenY)) (.z _relativelocation_2)) false false))
              (:Finished
                (Variables|Default|SetIsOpen true)))))))))

(event EventClose
  (bind _cube (Variables|Default|GetCube))
  (bind _cube_2 (Variables|Default|GetCube))
  (bind _cube_3 (Variables|Default|GetCube))
  (bind _cube_4 (Variables|Default|GetCube))
  (bind _relativelocation (Variables|/Script/Engine.SceneComponent|GetRelativeLocation _cube))
  (bind _relativelocation_2 (Variables|/Script/Engine.SceneComponent|GetRelativeLocation _cube_4))
  (bind _relativelocation_3 (Variables|/Script/Engine.SceneComponent|GetRelativeLocation _cube_2))
  (bind _relativelocation_4 (Variables|/Script/Engine.SceneComponent|GetRelativeLocation _cube_3))
  (if (Variables|Default|GetEnabled)
    (if (Variables|Default|GetIsOpen)
      (if (Variables|Default|GetIsExt)
        (bind _zeroto1 (Timeline|CloseY_2 Play)
          (:Update
            (Transformation|SetRelativeLocation _cube_4 (Math|Vector|MakeVector (.x _relativelocation_2) (Math|Float|Lerp _zeroto1 0.0 (Variables|Default|GetExtClosedY)) (.z _relativelocation_2)) false false))
          (:Finished
            (bind _1tozero (Timeline|CloseX_2 Play)
              (:Update
                (Transformation|SetRelativeLocation _cube (Math|Vector|MakeVector (Math|Float|Lerp _1tozero 0.0 (Variables|Default|GetExtClosedX)) (.y _relativelocation) (.z _relativelocation)) false false))
              (:Finished
                (Variables|Default|SetIsOpen false :!label _label)
                (Class|Door|OnDoorCloseComplete)))))
        (else
          (bind _zeroto1_2 (Timeline|CloseY_1 Play)
            (:Update
              (Transformation|SetRelativeLocation _cube_3 (Math|Vector|MakeVector (.x _relativelocation_4) (Math|Float|Lerp _zeroto1_2 0.0 (Variables|Default|GetIntOpenY)) (.z _relativelocation_4)) false false))
            (:Finished
              (bind _1tozero_2 (Timeline|CloseX_1 Play)
                (:Update
                  (Transformation|SetRelativeLocation _cube_2 (Math|Vector|MakeVector (Math|Float|Lerp _1tozero_2 0.0 (Variables|Default|GetIntOpenX)) (.y _relativelocation_3) (.z _relativelocation_3)) false false))
                (:Finished
                  (goto _label))))))))
    (else
      (Class|Door|OnDoorCloseComplete))))

(event EventBeginPlay)

(fn ConstructionScript)