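; StateTree evaluator for bots that tracks the location of the closest living player.
; On tree start it caches all LttnCharacter actors once and starts a looping 1.5-second timer.
; Each timer tick filters out invalid or dead players, finds the one nearest the Bot and stores its position in TargetLocation, leaving the last value when none remain.
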(event Custom|FindClosestPlayer
  (bind _activeplayers (CallFunction|GetActivePlayers))
  (if (not (Utilities|Array|IsEmpty _activeplayers))
    (Variables|Output|SetTargetLocation (Transformation|GetActorLocation (.ReturnValue (Actor|FindNearestActor (Transformation|GetActorLocation (Variables|Input|GetBot)) _activeplayers))))))

(event EventTreeStart
  (bind _outactors (Actor|GetAllActorsOfClass "/Script/Char0.LttnCharacter"))
  (Variables|Default|SetPlayers _outactors)
  (Utilities|Time|SetTimerbyEvent (delegate Custom|FindClosestPlayer) 1.5 true))

(fn GetActivePlayers
  (for _array_element (Variables|Default|GetPlayers)
    (Utilities|IsValid _array_element
      (:Is%20Valid
        (if (not (Variables|/Script/Char0.LttnCharacter|GetbIsDead _array_element))
          (Utilities|Array|Add (LocalVariables|GetActive) _array_element)))))
  (return (LocalVariables|GetActive)))