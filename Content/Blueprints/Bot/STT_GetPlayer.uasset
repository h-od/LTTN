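; A StateTree task for bots that picks the nearest living player as the bot's target and focus.
; On entering the state, it gathers player characters by PlayerArray index, filters out dead or invalid ones, then sets Target and controller focus to the closest.
; The search reruns inside the gathering loop, and a failed cast stops that path.
; A looping timer for periodic retargeting is unconnected, and its event is empty.
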(event Custom|FindClosestPlayer)

(event EventLatentEnterState
  (params (Transition :type State%20Tree%20Transition%20Result%20Structure%20%28by%20ref%29))
  ;[0.15 0.15 0.15 0.5] TODO if is single player, just return that. Need to find out how to update once it's passed
  (for (_ _array_index) (Variables|/Script/Engine.GameStateBase|GetPlayerArray (Game|GetGameState))
    (bind _aslttn_character (Utilities|Casting|CastToLttnCharacter (Game|Player|GetPlayerPawn _array_index)))
    (Utilities|Array|Add (Variables|Default|GetPlayers) _aslttn_character)
    (bind _activeplayers (CallFunction|GetActivePlayers))
    (Development|PrintString "Hello")
    (Utilities|IsValid (.ReturnValue (Actor|FindNearestActor (Transformation|GetActorLocation (Variables|Input|GetBot)) _activeplayers))
      (:Is%20Valid
        (Variables|Output|SetTarget (.ReturnValue (Actor|FindNearestActor (Transformation|GetActorLocation (Variables|Input|GetBot)) _activeplayers)))
        (AI|SetFocus (Variables|Context|GetController) (.ReturnValue (Actor|FindNearestActor (Transformation|GetActorLocation (Variables|Input|GetBot)) _activeplayers))))
      (:Is%20Not%20Valid
        (Development|PrintString "No Valid Char")))))

(fn GetActivePlayers
  (Utilities|Array|Clear (LocalVariables|GetActive))
  (for _array_element (Variables|Default|GetPlayers)
    (Utilities|IsValid _array_element
      (:Is%20Valid
        (if (not (Variables|/Script/Char0.LttnCharacter|GetbIsDead _array_element))
          (Utilities|Array|Add (LocalVariables|GetActive) _array_element)))))
  (return (LocalVariables|GetActive)))